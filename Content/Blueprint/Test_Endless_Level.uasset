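; Level tile for an endless side-scroller that randomizes its contents and exposes an attach point transform for chaining.
; Its construction script gathers left and right spawn points, adds blocker child actors at them, including a guarded left-side startup platform, and places a powerup randomly inside a box area.
; When the side-scroller character overlaps the end floor, it calls Add on the game mode, then destroys itself after a short delay.
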(event `self.EndFloor.OnComponentBeginOverlap`
  (params (OverlappedComponent :type "PrimitiveComponent Object Reference") (OtherActor :type "Actor Object Reference") (OtherComp :type "PrimitiveComponent Object Reference") (OtherBodyIndex :type Integer) (bFromSweep :type Boolean) (SweepResult :type "HitResult Structure (by ref)"))
  (cast `/Game/SideScrollerBP/Blueprints/SideScrollerCharacter` OtherActor)
  (bind _asside_scroller_game_mode (cast `/Game/SideScrollerBP/Blueprints/SideScrollerGameMode` (`GameplayStatics.GetGameMode`)))
  (`/Game/SideScrollerBP/Blueprints/SideScrollerGameMode.Add` _asside_scroller_game_mode)
  (`KismetSystemLibrary.Delay` 5.0)
  (`self.K2_DestroyActor`))

(fn `GetAttachTransform`
  (returns (AttachTransform :type "Transform Structure"))
  (return (`SceneComponent.K2_GetComponentToWorld` (`self.Attach Point`))))

(fn `SetSpawnPonts`
  (set `self.SpawnPonts` (`|MakeArray` (`SceneComponent.GetRelativeTransform` (`self.SpawnLeft`)) (`SceneComponent.GetRelativeTransform` (`self.SpawnRight`)))))

(fn `Spawn Blocker`
  (bind _spawnponts (`self.SpawnPonts`))
  (bind _spawnponts_2 (`self.SpawnPonts`))
  (while (`self.Do_Once`)
    (`AddComponent|NODE_AddChildActorComponent-1` :`RelativeTransform` (`|GetArrayItem` (`self.SpawnPonts`) (`KismetMathLibrary.RandomIntegerInRange` 0)))
    (set `self.Do_Once` false))
  (switch `int` (`KismetMathLibrary.RandomIntegerInRange` 0 4)
    (:`Default`
      (`AddComponent|NODE_AddChildActorComponent-2` :`RelativeTransform` (`|GetArrayItem` _spawnponts (`KismetMathLibrary.RandomIntegerInRange` 0 (`KismetArrayLibrary.Array_LastIndex` _spawnponts))) :!label _label))
    (:`0`
      (`AddComponent|NODE_AddChildActorComponent-3` :`RelativeTransform` (`|GetArrayItem` _spawnponts_2 (`KismetMathLibrary.RandomIntegerInRange` 0 (`KismetArrayLibrary.Array_LastIndex` _spawnponts_2)))))
    (:`1`
      (goto _label))
    (:`2`
      (goto _label))
    (:`3`
      (goto _label))
    (:`4`
      (goto _label))))

(fn `SpawnPowerups`
  (bind _possible_spawn_area (`self.Possible Spawn Area`))
  (`AddComponent|NODE_AddChildActorComponent-0` :`RelativeTransform` (`KismetMathLibrary.Conv_VectorToTransform` (`KismetMathLibrary.RandomPointInBoundingBox` (`SceneComponent.RelativeLocation` _possible_spawn_area) (`BoxComponent.GetScaledBoxExtent` _possible_spawn_area)))))

(fn `UserConstructionScript`
  (`self.SetSpawnPonts`)
  (`self.Spawn Blocker`)
  (`self.SpawnPowerups`))