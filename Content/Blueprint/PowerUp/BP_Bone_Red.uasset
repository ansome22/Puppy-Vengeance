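; BP_Bone_Red is a bone power-up pickup that awards points and temporarily changes the SideScrollerCharacter's bark.
; On overlap with that character, it adds points, plays a powerup sound, destroys itself, then calls BarkRadius.
; BarkRadius calls Bark with a raised value and uses a Delay to restore it, though this timer runs on the already destroyed actor.
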(event `self.ReceiveActorBeginOverlap`
  (params (OtherActor :type "Actor Object Reference"))
  (bind _asside_scroller_character (cast `/Game/SideScrollerBP/Blueprints/SideScrollerCharacter` OtherActor)) ; add event for power up
  (set `/Game/SideScrollerBP/Blueprints/SideScrollerCharacter.Points` (+ (`/Game/SideScrollerBP/Blueprints/SideScrollerCharacter.Points` _asside_scroller_character) 10) _asside_scroller_character)
  (`GameplayStatics.PlaySoundAtLocation` "/Game/Sound/SFX_Powerup_01.SFX_Powerup_01" (`self.K2_GetActorLocation`)) ; sound is in root/Sound folder
  (`self.K2_DestroyActor`)
  (`self.Bark Radius`))

(event `Bark Radius`
  ;[1 1 1] Bark
  (bind _asside_scroller_character (cast `/Game/SideScrollerBP/Blueprints/SideScrollerCharacter` (stale `self.ReceiveActorBeginOverlap` OtherActor)))
  (`/Game/SideScrollerBP/Blueprints/SideScrollerCharacter.Bark` _asside_scroller_character 2)
  (`KismetSystemLibrary.Delay` 6.0)
  (`/Game/SideScrollerBP/Blueprints/SideScrollerCharacter.Bark` _asside_scroller_character 1))

(fn `UserConstructionScript`)