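; Enemy that turns toward the player and throws YarnBall projectiles when its PawnSensing component sees a pawn.
; Each sighting sets yaw and roll via RInterpTo from the seen pawn's rotation toward player 0, with pitch zeroed.
; A Delay then throttles FireAtPlayer, which spawns a YarnBall ahead along control rotation, using the same interpolated aim.
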(event `self.PawnSensing.OnSeePawn`
  (params (Pawn :type "Pawn Object Reference"))
  (`self.K2_SetActorRotation` (`KismetMathLibrary.RInterpTo` (`self.K2_GetActorRotation` Pawn) (`KismetMathLibrary.MakeRotator` (.roll (`KismetMathLibrary.FindLookAtRotation` (`self.K2_GetActorLocation`) (`self.K2_GetActorLocation` (`GameplayStatics.GetPlayerCharacter` 0)))) 0.0 (.yaw (`KismetMathLibrary.FindLookAtRotation` (`self.K2_GetActorLocation`) (`self.K2_GetActorLocation` (`GameplayStatics.GetPlayerCharacter` 0))))) (`GameplayStatics.GetWorldDeltaSeconds`) 300.0))
  (`KismetSystemLibrary.Delay` 2.2)
  (`self.Fire At Player`))

(event `Fire At Player`
  (`|SpawnActorFromClass` "/Game/Blueprint/Enemy/YarnBall.YarnBall_C" (`KismetMathLibrary.MakeTransform` (+ (`self.K2_GetActorLocation`) (* (`KismetMathLibrary.GetForwardVector` (`self.GetControlRotation`)) 50.0)) (`KismetMathLibrary.RInterpTo` (`self.K2_GetActorRotation` (stale `self.PawnSensing.OnSeePawn` Pawn)) (`KismetMathLibrary.MakeRotator` (.roll (`KismetMathLibrary.FindLookAtRotation` (`self.K2_GetActorLocation`) (`self.K2_GetActorLocation` (`GameplayStatics.GetPlayerCharacter` 0)))) 0.0 (.yaw (`KismetMathLibrary.FindLookAtRotation` (`self.K2_GetActorLocation`) (`self.K2_GetActorLocation` (`GameplayStatics.GetPlayerCharacter` 0))))) (`GameplayStatics.GetWorldDeltaSeconds`) 300.0)) "Undefined" "OverrideRootScale"))

(fn `UserConstructionScript`)