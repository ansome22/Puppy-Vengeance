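; Floor tile for an endless side-scroller level, exposing an attach-point transform for chaining tiles.
; Its construction script randomly adds child actors: a blocker or occasional enemy at the left or right spawn point, and sometimes a powerup inside the spawn box.
; When the player character overlaps EndFloor, it calls Add on the game mode, then destroys itself after a delay.
; SpawnEnemy is an empty stub.
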(event `self.EndFloor.OnComponentBeginOverlap`
  (params (OverlappedComponent :type "PrimitiveComponent Object Reference") (OtherActor :type "Actor Object Reference") (OtherComp :type "PrimitiveComponent Object Reference") (OtherBodyIndex :type Integer) (bFromSweep :type Boolean) (SweepResult :type "HitResult Structure (by ref)"))
  (cast `/Game/SideScrollerBP/Blueprints/SideScrollerCharacter` OtherActor)
  (bind _asside_scroller_game_mode (cast `/Game/SideScrollerBP/Blueprints/SideScrollerGameMode` (`GameplayStatics.GetGameMode`)))
  (`/Game/SideScrollerBP/Blueprints/SideScrollerGameMode.Add` _asside_scroller_game_mode)
  (`KismetSystemLibrary.Delay` 10.0)
  (`self.K2_DestroyActor`))

(fn `GetAttachTransform`
  (returns (AttachTransform :type "Transform Structure"))
  (return (`SceneComponent.K2_GetComponentToWorld` (`self.Attach Point`))))

(fn `SetSpawnPonts`
  (set `self.SpawnPonts` (`|MakeArray` (`SceneComponent.GetRelativeTransform` (`self.SpawnLeft`)) (`SceneComponent.GetRelativeTransform` (`self.SpawnRight`)))))

(fn `Spawn Blocker`
  (bind _spawnponts (`self.SpawnPonts`))
  (bind _spawnponts_2 (`self.SpawnPonts`))
  (switch `int` (`KismetMathLibrary.RandomIntegerInRange` 0 4)
    (:`Default`
      (`AddComponent|NODE_AddChildActorComponent-2` :`RelativeTransform` (`|GetArrayItem` _spawnponts (`KismetMathLibrary.RandomIntegerInRange` 0 (`KismetArrayLibrary.Array_LastIndex` _spawnponts))) :!label _label))
    (:`0`
      (bind _output_get (set `self.test` (`|GetArrayItem` _spawnponts_2 (`KismetMathLibrary.RandomIntegerInRange` 0 (`KismetArrayLibrary.Array_LastIndex` _spawnponts_2)))))
      (`AddComponent|NODE_AddChildActorComponent-3` :`RelativeTransform` _output_get) ; Enemy
    )
    (:`1`
      (goto _label))
    (:`2`
      (goto _label))
    (:`3`
      (goto _label))
    (:`4`
      (goto _label))))

(fn `Spawn Enemy`)

(fn `SpawnPowerups`
  (bind _possible_spawn_area (`self.Possible Spawn Area`))
  (bind _returnvalue (`KismetMathLibrary.Conv_VectorToTransform` (`KismetMathLibrary.TransformLocation` (`SceneComponent.K2_GetComponentToWorld` _possible_spawn_area) (`KismetMathLibrary.RandomPointInBoundingBox` (0.0 0.0 0.0) (`BoxComponent.BoxExtent` _possible_spawn_area)))))
  (switch `int` (`KismetMathLibrary.RandomIntegerInRange` 0 5)
    (:`0`
      (`AddComponent|NODE_AddChildActorComponent-0` :`RelativeTransform` _returnvalue))
    (:`1`
      (`AddComponent|NODE_AddChildActorComponent-4` :`RelativeTransform` _returnvalue))
    (:`2`
      (`AddComponent|NODE_AddChildActorComponent-5` :`RelativeTransform` _returnvalue))))

(fn `UserConstructionScript`
  (`self.SetSpawnPonts`)
  (`self.Spawn Blocker`)
  (`self.Spawn Enemy`)
  (`self.SpawnPowerups`))